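; Trigger actor that toggles AI control of every BP_Enemy, switching it off at BeginPlay and flipping it each time BP_ThirdPersonCharacter overlaps its Box.
; A FlipFlop alternates two passes: the first clears the SeesPlayer blackboard key, stops movement, stores each AI controller and unpossesses it.
; The second repossesses enemies from TempAiController by array index, relying on matching actor order; the array is never cleared.
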(event OnComponentBeginOverlap(Box)
  (params (OverlappedComponent :type Primitive%20Component%20Object%20Reference) (OtherActor :type Actor%20Object%20Reference) (OtherComp :type Primitive%20Component%20Object%20Reference) (OtherBodyIndex :type Integer) (bFromSweep :type Boolean) (SweepResult :type Hit%20Result%20Structure%20%28by%20ref%29))
  (Utilities|Casting|CastToBP_ThirdPersonCharacter OtherActor)
  (Utilities|FlowControl|FlipFlop
    (:A
      (bind _outactors (Actor|GetAllActorsOfClass "/Game/AI/BP_Enemy.BP_Enemy_C"))
      (for _array_element _outactors
        (AI|Components|Blackboard|SetValueasBool (AI|GetBlackboard _array_element) (Utilities|Name|MakeLiteralName "SeesPlayer") false)
        (Components|Movement|StopMovementImmediately (Variables|/Script/Engine.Character|GetCharacterMovement _array_element))
        (Utilities|Array|Add (Variables|Default|GetTempAiController) (AI|GetAIController _array_element))
        (Pawn|UnPossess (AI|GetAIController _array_element))))
    (:B
      (bind _outactors_2 (Actor|GetAllActorsOfClass "/Game/AI/BP_Enemy.BP_Enemy_C"))
      (for (_array_element_2 _array_index) _outactors_2
        (Pawn|Possess (Utilities|Array|Get(acopy) (Variables|Default|GetTempAiController) _array_index) _array_element_2)))))

(event Custom|ToogleAI
  (Utilities|FlowControl|FlipFlop
    (:A
      (bind _outactors (Actor|GetAllActorsOfClass "/Game/AI/BP_Enemy.BP_Enemy_C"))
      (for _array_element _outactors
        (AI|Components|Blackboard|SetValueasBool (AI|GetBlackboard _array_element) (Utilities|Name|MakeLiteralName "SeesPlayer") false)
        (Components|Movement|StopMovementImmediately (Variables|/Script/Engine.Character|GetCharacterMovement _array_element))
        (Utilities|Array|Add (Variables|Default|GetTempAiController) (AI|GetAIController _array_element))
        (Pawn|UnPossess (AI|GetAIController _array_element))))
    (:B
      (bind _outactors_2 (Actor|GetAllActorsOfClass "/Game/AI/BP_Enemy.BP_Enemy_C"))
      (for (_array_element_2 _array_index) _outactors_2
        (Pawn|Possess (Utilities|Array|Get(acopy) (Variables|Default|GetTempAiController) _array_index) _array_element_2)))))

(event EventBeginPlay
  (Utilities|FlowControl|FlipFlop
    (:A
      (bind _outactors (Actor|GetAllActorsOfClass "/Game/AI/BP_Enemy.BP_Enemy_C"))
      (for _array_element _outactors
        (AI|Components|Blackboard|SetValueasBool (AI|GetBlackboard _array_element) (Utilities|Name|MakeLiteralName "SeesPlayer") false)
        (Components|Movement|StopMovementImmediately (Variables|/Script/Engine.Character|GetCharacterMovement _array_element))
        (Utilities|Array|Add (Variables|Default|GetTempAiController) (AI|GetAIController _array_element))
        (Pawn|UnPossess (AI|GetAIController _array_element))))
    (:B
      (bind _outactors_2 (Actor|GetAllActorsOfClass "/Game/AI/BP_Enemy.BP_Enemy_C"))
      (for (_array_element_2 _array_index) _outactors_2
        (Pawn|Possess (Utilities|Array|Get(acopy) (Variables|Default|GetTempAiController) _array_index) _array_element_2)))))

(fn ConstructionScript)